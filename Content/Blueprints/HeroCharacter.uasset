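; Player hero character for a twin-stick shooter, handling weapon fire, death with respawn, and power feedback.
; BeginPlay attaches a spawned weapon to GunSocket, records the spawn transform in TwinStickMode and adds the HUD; left mouse drives the trigger.
; On death, it disables input, waits, requests a respawn and destroys itself and its weapon.
; Power changes tint the body through a dynamic material created in the construction script.
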(event `self.ReceiveBeginPlay`
  (bind _mesh (`self.Mesh`))
  (`|ExecutionSequence`
    (:`then_0`
      (bind _returnvalue (`|SpawnActorFromClass` "/Game/Blueprints/Weapon.Weapon_C" (`SceneComponent.K2_GetComponentToWorld` _mesh) "Undefined" "OverrideRootScale"))
      (bind _output_get (set `self.Weapon` _returnvalue))
      (`self.K2_AttachRootComponentTo` _output_get _mesh "GunSocket" "SnapToTarget" true))
    (:`then_1`
      (bind _astwin_stick_mode (cast `/Game/Blueprints/TwinStickMode` (`GameplayStatics.GetGameMode`)))
      (bind _output_get_2 (set `self.GameMode` _astwin_stick_mode))
      (set `/Game/Blueprints/TwinStickMode.PlayerSpawnTransform` (`self.GetTransform`) _output_get_2))
    (:`then_2`
      (bind _returnvalue_2 (`|CreateWidget` "/Game/Blueprints/TwinStickHUD.TwinStickHUD_C"))
      (`UserWidget.AddToViewport` _returnvalue_2 0))))

(event `Key|LeftMouseButton`
  (params (Key :type "Key Structure" :default "AnyKey"))
  (bind _weapon (`self.Weapon`))
  (:`Pressed`
    (`/Game/Blueprints/Weapon.PullTrigger` _weapon))
  (:`Released`
    (`/Game/Blueprints/Weapon.ReleaseTrigger` _weapon)))

(event `/Game/Blueprints/iDamageable.AffectHealth`
  (params (Delta :type "Float (single-precision)"))
  (`self.CalculateHealth` Delta)
  (if (`self.isDead`)
    (`self.DisableInput` null)
    (`KismetSystemLibrary.Delay` 3.0)
    (`/Game/Blueprints/TwinStickMode.RespawnPlayer` (`self.GameMode`))
    (`self.K2_DestroyActor` (`self.Weapon`))
    (`self.K2_DestroyActor` self)))

(event `self.PowerChangeEffect`
  (`MaterialInstanceDynamic.SetVectorParameterValue` (`self.PowerMaterial`) "BodyColor" (`KismetMathLibrary.LinearColorLerp` (struct :`R` 0.285 :`G` 0.786 :`B` 1.0 :`A` 1.0) (struct :`R` 0.74 :`G` 0.36 :`B` 0.02812 :`A` 1.0) (`KismetMathLibrary.FClamp` (/ (`self.GetCurrentPower`) (`self.GetInitialPower`))))))

(fn `UserConstructionScript`
  (bind _mesh (`self.Mesh`))
  (bind _returnvalue (`PrimitiveComponent.CreateDynamicMaterialInstance` _mesh 0 (`KismetArrayLibrary.Array_Get` (`MeshComponent.GetMaterials` _mesh))))
  (set `self.PowerMaterial` _returnvalue))